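; BP_squadmanager coordinates which volleyball character goes for the ball, based on where it will land and who touched it last.
; CheckBallImpact predicts the physics ball's path, clamps the impact to the court and clears previous orders.
; After an opponent AI touch, the closer of player or AI teammate moves there, projected onto the navmesh.
; Otherwise an opponent is picked by distance, while unordered ones get a blackboard phase and fixed pass location.
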(fn ConstructionScript)

(fn CheckBallImpact
  (params (callbycounter :type Boolean))
  (bind _outactors (Actor|GetAllActorsOfClass "/Game/BP_Class/BP_Ball.BP_Ball_C"))
  (if (> (Utilities|Array|Length _outactors) 0)
    (bind _output_get (Variables|Default|SetBallref (Utilities|Array|Get(acopy) _outactors)))
    (bind _output_get_2 (Variables|Default|SetBallMesh (Actor|GetComponentbyClass _output_get "/Script/Engine.StaticMeshComponent")))
    (if (Physics|IsSimulatingPhysics _output_get_2 "None")
      (bind _returnvalue (Physics|GetPhysicsLinearVelocity (Variables|Default|GetBallMesh) "None"))
      (bind _predictresult (Class|GameplayStatics|BlueprintPredictProjectilePathAdvanced (Utilities|Struct|MakePredictProjectilePathParams (Transformation|GetWorldLocation (Variables|Default|GetBallMesh)) _returnvalue true 15.0 4.0 true "ECC_Visibility" "ObjectTypeQuery1" (Utilities|Array|MakeArray (Variables|Default|GetBallref)) 3e+01)))
      (bind _output_get_3 (Variables|Default|SetImpactraw (Math|Vector|SelectVector (.Location (Collision|BreakHitResult (.HitResult (Utilities|Struct|BreakPredictProjectilePathResult _predictresult)))) (.Location (Utilities|Struct|BreakPredictProjectilePathPointData (.LastTraceDestination (Utilities|Struct|BreakPredictProjectilePathResult _predictresult)))) (.bBlockingHit (Collision|BreakHitResult (.HitResult (Utilities|Struct|BreakPredictProjectilePathResult _predictresult)))))))
      (Variables|Default|Setimpactpoint (Math|Vector|MakeVector (Math|Float|Clamp(Float) (.X (Math|Vector|BreakVector _output_get_3)) (Variables|Default|GetCourminX) (Variables|Default|GetCourMaxX)) (Math|Float|Clamp(Float) (.Y (Math|Vector|BreakVector _output_get_3)) (Variables|Default|GetCourMinY) (Variables|Default|GetCourMaxY)) (Variables|Default|GetCourtZ)))
      (bind _outactors_2 (Actor|GetAllActorsOfClass "/Game/BP_Class/BP_ScoreManager.BP_ScoreManager_C"))
      (CallFunction|RemoveAI)
      (Utilities|Casting|CastToBP_AI (Variables|/Game/BP_Class/BP_ScoreManager.BP_ScoreManager_C|GetPlayerLastTouch (Utilities|Array|Get(acopy) _outactors_2))
        (:then
          (Rendering|Debug|DrawDebugSphere (Variables|Default|Getimpactpoint) 3e+01 50 "(R=1.000000,G=0.000000,B=0.095176,A=1.000000)" 0.1)
          (bind _outactors_3 (Actor|GetAllActorsOfClass "/Game/ThirdPerson/Blueprints/BP_Player.BP_Player_C"))
          (bind _outactors_4 (Actor|GetAllActorsOfClass "/Game/ThirdPerson/Blueprints/BP_AIFriend.BP_AIFriend_C"))
          (Default|AIClearorder (Utilities|Array|Get(acopy) _outactors_4))
          (bind _output_get_4 (LocalVariables|Setcloseallie (Utilities|Array|Get(acopy) _outactors_4)))
          (if (> (Math|Vector|Distance(Vector) (Transformation|GetActorLocation (Utilities|Array|Get(acopy) _outactors_3)) (Variables|Default|Getimpactpoint)) (Math|Vector|Distance(Vector) (Transformation|GetActorLocation (Utilities|Array|Get(acopy) _outactors_4)) (Variables|Default|Getimpactpoint)))
            (Variables|/Game/ThirdPerson/Blueprints/BP_AIFriend.BP_AIFriend_C|SetHasorder _output_get_4 true)
            (Default|AISetGoal _output_get_4 (Math|Vector|SelectVector (.ProjectedLocation (AI|Navigation|ProjectPointtoNavigation (Variables|Default|Getimpactpoint) 0 0 "0, 0, 0")) (Variables|Default|Getimpactpoint) (.ReturnValue (AI|Navigation|ProjectPointtoNavigation (Variables|Default|Getimpactpoint) 0 0 "0, 0, 0"))))
            (else
              (Variables|/Game/ThirdPerson/Blueprints/BP_Player.BP_Player_C|SetPlayeurMove (Utilities|Array|Get(acopy) _outactors_3) (Math|Vector|SelectVector (.ProjectedLocation (AI|Navigation|ProjectPointtoNavigation (Variables|Default|Getimpactpoint) 0 0 "0, 0, 0")) (Variables|Default|Getimpactpoint) (.ReturnValue (AI|Navigation|ProjectPointtoNavigation (Variables|Default|Getimpactpoint) 0 0 "0, 0, 0"))))
              (Default|Moveto (Utilities|Array|Get(acopy) _outactors_3)))))
        (:CastFailed
          (Utilities|Casting|CastToBP_Player (Variables|/Game/BP_Class/BP_ScoreManager.BP_ScoreManager_C|GetPlayerLastTouch (Utilities|Array|Get(acopy) _outactors_2))
            (:then
              _)
            (:CastFailed
              (Utilities|Casting|CastToBP_AIFriend (Variables|/Game/BP_Class/BP_ScoreManager.BP_ScoreManager_C|GetPlayerLastTouch (Utilities|Array|Get(acopy) _outactors_2)))))
          (bind _outactors_5 (Actor|GetAllActorsOfClass "/Game/ThirdPerson/Blueprints/BP_AI.BP_AI_C"))
          (for _array_element _outactors_5
            (Default|AIClearorder _array_element)
            (if (> (LocalVariables|GetBestDist) (Math|Vector|Distance(Vector) (Transformation|GetActorLocation _array_element) (Variables|Default|Getimpactpoint)))
              (LocalVariables|SetBestDist (Math|Vector|Distance(Vector) (Transformation|GetActorLocation _array_element) (Variables|Default|Getimpactpoint)))
              (bind _output_get_5 (Variables|Default|SetBestAI _array_element))))
          (bind _output_get_6 (LocalVariables|SetCLoseAI _output_get_5))
          (if (Math|Boolean|ANDBoolean (== (Math|Byte|MakeLiteralByte (Utilities|Enum|LiteralenumE_VolleyPhase "NewEnumerator3")) (Class|BlackboardComponent|GetValueasEnum (AI|GetBlackboard (Pawn|GetController _output_get_6)) (Utilities|Name|MakeLiteralName "EVolleyPhase"))) callbycounter true)
            (bind _outactors_6 (Actor|GetAllActorsOfClass "/Game/ThirdPerson/Blueprints/BP_AI.BP_AI_C"))
            (for _array_element_2 _outactors_6
              (Default|AIClearorder _array_element_2)
              (if (not (> (LocalVariables|GetBestDist) (Math|Vector|Distance(Vector) (Transformation|GetActorLocation _array_element_2) (Variables|Default|Getimpactpoint))))
                (LocalVariables|SetBestDist (Math|Vector|Distance(Vector) (Transformation|GetActorLocation _array_element_2) (Variables|Default|Getimpactpoint)))
                (bind _output_get_7 (Variables|Default|SetBestAI _array_element_2))))
            (LocalVariables|SetCLoseAI _output_get_7)
            (else
              (Variables|/Game/ThirdPerson/Blueprints/BP_AI.BP_AI_C|SetHasOrder (LocalVariables|GetCLoseAI) true)))
          (Variables|/Game/ThirdPerson/Blueprints/BP_AI.BP_AI_C|SetHasOrder (LocalVariables|GetCLoseAI) true)
          (bind _outactors_7 (Actor|GetAllActorsOfClass "/Game/ThirdPerson/Blueprints/BP_AI.BP_AI_C"))
          (for _array_element_3 _outactors_7
            (if (not (Variables|/Game/ThirdPerson/Blueprints/BP_AI.BP_AI_C|GetHasOrder _array_element_3))
              (bind _asaic_volley (Utilities|Casting|CastToAIC_Volley (Pawn|GetController _array_element_3)))
              (AI|Components|Blackboard|SetValueasEnum (AI|GetBlackboard _asaic_volley) (Utilities|Name|MakeLiteralName "EVolleyPhase") (Utilities|Enum|LiteralenumE_VolleyPhase "NewEnumerator2"))
              (AI|Components|Blackboard|SetValueasVector (AI|GetBlackboard _asaic_volley) (Utilities|Name|MakeLiteralName "PassLoc") "6914.527781,-145.844626,2450.999984")
              (Rendering|Debug|DrawDebugSphere (Variables|Default|Getimpactpoint) 3e+01 50 "(R=1.000000,G=0.000000,B=0.095176,A=1.000000)" 1.0)
              (Default|AISetGoal (LocalVariables|GetCLoseAI) (Math|Vector|SelectVector (.ProjectedLocation (AI|Navigation|ProjectPointtoNavigation (Variables|Default|Getimpactpoint) 0 0 "0, 0, 0")) (Variables|Default|Getimpactpoint) (.ReturnValue (AI|Navigation|ProjectPointtoNavigation (Variables|Default|Getimpactpoint) 0 0 "0, 0, 0")))))))))))

(fn RemoveAI
  (bind _outactors (Actor|GetAllActorsOfClass "/Game/ThirdPerson/Blueprints/BP_AIFriend.BP_AIFriend_C"))
  (Variables|/Game/ThirdPerson/Blueprints/BP_AIFriend.BP_AIFriend_C|SetHasorder (Utilities|Array|Get(acopy) _outactors) false)
  (bind _outactors_2 (Actor|GetAllActorsOfClass "/Game/ThirdPerson/Blueprints/BP_AI.BP_AI_C"))
  (for _array_element _outactors_2
    (Variables|/Game/ThirdPerson/Blueprints/BP_AI.BP_AI_C|SetHasOrder _array_element false)))