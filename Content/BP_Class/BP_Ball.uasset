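; Ball actor for a two-team court game that detects where it lands and awards points through BP_ScoreManager.
; Physics, gravity and collision start disabled at BeginPlay.
; Overlapping BP_CourtSide while BallLive scores that side's TeamId; BP_courtOut picks the team from PlayerLastTouch (AI or not), bypassing the BallLive check.
; Both paths share a delayed AddPoint call, guarded by a time cooldown against repeat scoring.
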(event OnComponentBeginOverlap(StaticMesh)
  (params (OverlappedComponent :type Primitive%20Component%20Object%20Reference) (OtherActor :type Actor%20Object%20Reference) (OtherComp :type Primitive%20Component%20Object%20Reference) (OtherBodyIndex :type Integer) (bFromSweep :type Boolean) (SweepResult :type Hit%20Result%20Structure%20%28by%20ref%29))
  ;[0.15 0.15 0.15 0.5] Systeme de scoring
  (bind _asbp_court_side (Utilities|Casting|CastToBP_CourtSide OtherActor)
    (:then
      (Variables|Default|SetTeamId (Variables|/Game/BP_Class/BP_CourtSide.BP_CourtSide_C|GetTeamid _asbp_court_side))
      (if (Variables|Default|GetBallLive)
        (bind _outactors (Actor|GetAllActorsOfClass "/Game/BP_Class/BP_ScoreManager.BP_ScoreManager_C" :!label _label))
        (if (> (Utilities|Array|Length _outactors) 0)
          (Variables|Default|SetScoreManagerRef (Utilities|Array|Get(acopy) _outactors))
          (Utilities|FlowControl|Delay 0.5)
          (if (> (- (Utilities|Time|GetGameTimeinSeconds) (Variables|Default|GetactionlastTime)) 3.0)
            (Default|AddPoint (Variables|Default|GetScoreManagerRef) (Variables|Default|GetTeamId))
            (Variables|Default|SetactionlastTime (Utilities|Time|GetGameTimeinSeconds))))))
    (:CastFailed
      (Utilities|Casting|CastToBP_courtOut OtherActor)
      (bind _outactors_2 (Actor|GetAllActorsOfClass "/Game/BP_Class/BP_ScoreManager.BP_ScoreManager_C"))
      (Variables|Default|SetScoreManagerRef (Utilities|Array|Get(acopy) _outactors_2))
      (Utilities|Casting|CastToBP_AI (Variables|/Game/BP_Class/BP_ScoreManager.BP_ScoreManager_C|GetPlayerLastTouch (Utilities|Array|Get(acopy) _outactors_2))
        (:then
          (Variables|Default|SetTeamId 1)
          (goto _label))
        (:CastFailed
          (Variables|Default|SetTeamId 0)
          (goto _label))))))

(event EventBeginPlay
  (bind _staticmesh (Variables|Default|GetStaticMesh))
  ;[0.15 0.15 0.15 0.5] Ajout de classe de scoring
  (bind _outactors (Actor|GetAllActorsOfClass "/Game/BP_Class/BP_ScoreManager.BP_ScoreManager_C"))
  (Variables|Default|SetScoreManagerRef 0)
  ;[0.15 0.15 0.15 0.5] desactivation de la physique et des collision de la balle en debut de set
  (Physics|SetSimulatePhysics _staticmesh false)
  (Physics|SetEnableGravity _staticmesh false)
  (Collision|SetCollisionEnabled _staticmesh "NoCollision"))

(fn ConstructionScript)