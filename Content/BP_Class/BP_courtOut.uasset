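; BP_courtOut is an out-of-bounds detector that reacts when the ball leaves the court.
; Four trigger components (top, bottom, left and right) filter overlaps for BP_Ball and share one handler.
; The handler prints a debug message, looks up all BP_Player actors and sets the ServiceEtat of only the first one found to NewEnumerator0.
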(event OnComponentBeginOverlap(OutTop)
  (params (OverlappedComponent :type Primitive%20Component%20Object%20Reference) (OtherActor :type Actor%20Object%20Reference) (OtherComp :type Primitive%20Component%20Object%20Reference) (OtherBodyIndex :type Integer) (bFromSweep :type Boolean) (SweepResult :type Hit%20Result%20Structure%20%28by%20ref%29))
  (Utilities|Casting|CastToBP_Ball OtherActor)
  (Development|PrintString "ball out")
  (bind _outactors (Actor|GetAllActorsOfClass "/Game/ThirdPerson/Blueprints/BP_Player.BP_Player_C"))
  (Variables|/Game/ThirdPerson/Blueprints/BP_Player.BP_Player_C|SetServiceEtat (Utilities|Array|Get(acopy) _outactors) "NewEnumerator0"))

(event OnComponentBeginOverlap(OurBottom)
  (params (OverlappedComponent :type Primitive%20Component%20Object%20Reference) (OtherActor :type Actor%20Object%20Reference) (OtherComp :type Primitive%20Component%20Object%20Reference) (OtherBodyIndex :type Integer) (bFromSweep :type Boolean) (SweepResult :type Hit%20Result%20Structure%20%28by%20ref%29))
  (Utilities|Casting|CastToBP_Ball OtherActor)
  (Development|PrintString "ball out")
  (bind _outactors (Actor|GetAllActorsOfClass "/Game/ThirdPerson/Blueprints/BP_Player.BP_Player_C"))
  (Variables|/Game/ThirdPerson/Blueprints/BP_Player.BP_Player_C|SetServiceEtat (Utilities|Array|Get(acopy) _outactors) "NewEnumerator0"))

(event OnComponentBeginOverlap(OutLeft)
  (params (OverlappedComponent :type Primitive%20Component%20Object%20Reference) (OtherActor :type Actor%20Object%20Reference) (OtherComp :type Primitive%20Component%20Object%20Reference) (OtherBodyIndex :type Integer) (bFromSweep :type Boolean) (SweepResult :type Hit%20Result%20Structure%20%28by%20ref%29))
  (Utilities|Casting|CastToBP_Ball OtherActor)
  (Development|PrintString "ball out")
  (bind _outactors (Actor|GetAllActorsOfClass "/Game/ThirdPerson/Blueprints/BP_Player.BP_Player_C"))
  (Variables|/Game/ThirdPerson/Blueprints/BP_Player.BP_Player_C|SetServiceEtat (Utilities|Array|Get(acopy) _outactors) "NewEnumerator0"))

(event OnComponentBeginOverlap(OutRight)
  (params (OverlappedComponent :type Primitive%20Component%20Object%20Reference) (OtherActor :type Actor%20Object%20Reference) (OtherComp :type Primitive%20Component%20Object%20Reference) (OtherBodyIndex :type Integer) (bFromSweep :type Boolean) (SweepResult :type Hit%20Result%20Structure%20%28by%20ref%29))
  (Utilities|Casting|CastToBP_Ball OtherActor)
  (Development|PrintString "ball out")
  (bind _outactors (Actor|GetAllActorsOfClass "/Game/ThirdPerson/Blueprints/BP_Player.BP_Player_C"))
  (Variables|/Game/ThirdPerson/Blueprints/BP_Player.BP_Player_C|SetServiceEtat (Utilities|Array|Get(acopy) _outactors) "NewEnumerator0"))

(event EventTick
  (params (DeltaSeconds :type Float%20%28single-precision%29)))

(event EventBeginPlay)

(fn ConstructionScript)