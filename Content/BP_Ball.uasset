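; BP_Ball is a ball with a court-side scoring system, launched by the IA_Service input enabling physics, gravity and collision.
; When the mesh overlaps a BP_CourtSide while BallLive and its Z velocity is below 100, it passes that side's Teamid to BP_ScoreManager's AddPoint.
; BeginPlay leaves the manager reference empty, so the overlap looks it up; the physics-disabling nodes never run.
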(event OnComponentBeginOverlap(StaticMesh)
  (params (OverlappedComponent :type Primitive%20Component%20Object%20Reference) (OtherActor :type Actor%20Object%20Reference) (OtherComp :type Primitive%20Component%20Object%20Reference) (OtherBodyIndex :type Integer) (bFromSweep :type Boolean) (SweepResult :type Hit%20Result%20Structure%20%28by%20ref%29))
  ;[0.15 0.15 0.15 0.5] Systeme de scoring
  (bind _returnvalue (Physics|GetPhysicsLinearVelocity (Variables|Default|GetStaticMesh) "None"))
  (if (Variables|Default|GetBallLive)
    (if (< (.Z (Math|Vector|BreakVector _returnvalue)) 1e+02)
      (Development|PrintString "detection de la balle")
      (bind _asbp_court_side (Utilities|Casting|CastToBP_CourtSide OtherActor))
      (bind _outactors (Actor|GetAllActorsOfClass "/Game/BP_ScoreManager.BP_ScoreManager_C"))
      (if (> (Utilities|Array|Length _outactors) 0)
        (bind _output_get (Variables|Default|SetScoreManagerRef (Utilities|Array|Get(acopy) _outactors)))
        (Default|AddPoint _output_get (Variables|/Game/BP_CourtSide.BP_CourtSide_C|GetTeamid _asbp_court_side))
        (Development|PrintString "function d'ajout appeler")))))

(event Input|EnhancedActionEvents|EnhancedInputActionIA_Service
  (params (ActionValue :type Boolean) (ElapsedSeconds :type Float%20%28double-precision%29) (TriggeredSeconds :type Float%20%28double-precision%29) (InputAction :type Input%20Action%20Object%20Reference :default "/Game/ThirdPerson/Input/Actions/IA_Service.IA_Service"))
  (bind _staticmesh (Variables|Default|GetStaticMesh))
  (Physics|SetSimulatePhysics _staticmesh true)
  (Physics|SetEnableGravity _staticmesh true)
  (Collision|SetCollisionEnabled _staticmesh "QueryAndPhysics"))

(event EventBeginPlay
  ;[0.15 0.15 0.15 0.5] Ajout de classe de scoring
  (bind _outactors (Actor|GetAllActorsOfClass "/Game/BP_ScoreManager.BP_ScoreManager_C"))
  (Variables|Default|SetScoreManagerRef 0))

(fn ConstructionScript)