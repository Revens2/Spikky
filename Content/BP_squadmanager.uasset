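; Squad manager for a ball court game that sends AI players to where the ball will land.
; It predicts the simulated ball's path and clamps the impact point to court bounds.
; CheckBallImpact clears orders, then uses the score manager's NextTeam to move either the friendly AI, when closer than the player, or the nearest opponent AI to that nav-projected point.
; Two variant functions handle each side separately, with debug spheres marking the target.
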(fn ConstructionScript)

(fn NewFunction
  (bind _returnvalue (Actor|GetActorOfClass "/Game/BP_ScoreManager.BP_ScoreManager_C"))
  (bind _returnvalue_2 (Physics|GetPhysicsLinearVelocity (Variables|/Game/BP_Ball.BP_Ball_C|GetStaticMesh (Variables|/Game/BP_ScoreManager.BP_ScoreManager_C|GetInball _returnvalue)) "None")))

(fn CheckBallImpact
  (bind _outactors (Actor|GetAllActorsOfClass "/Game/BP_Ball.BP_Ball_C"))
  (if (> (Utilities|Array|Length _outactors) 0)
    (bind _output_get (Variables|Default|SetBallref (Utilities|Array|Get(acopy) _outactors)))
    (bind _output_get_2 (Variables|Default|SetBallMesh (Actor|GetComponentbyClass _output_get "/Script/Engine.StaticMeshComponent")))
    (if (Physics|IsSimulatingPhysics _output_get_2 "None")
      (bind _returnvalue (Physics|GetPhysicsLinearVelocity (Variables|Default|GetBallMesh) "None"))
      (bind _predictresult (Class|GameplayStatics|BlueprintPredictProjectilePathAdvanced (Utilities|Struct|MakePredictProjectilePathParams (Transformation|GetWorldLocation (Variables|Default|GetBallMesh)) _returnvalue true 15.0 4.0 true "ECC_Visibility" "ObjectTypeQuery1" (Utilities|Array|MakeArray (Variables|Default|GetBallref)) 3e+01)))
      (bind _output_get_3 (Variables|Default|SetImpactraw (Math|Vector|SelectVector (.Location (Collision|BreakHitResult (.HitResult (Utilities|Struct|BreakPredictProjectilePathResult _predictresult)))) (.Location (Utilities|Struct|BreakPredictProjectilePathPointData (.LastTraceDestination (Utilities|Struct|BreakPredictProjectilePathResult _predictresult)))) (.bBlockingHit (Collision|BreakHitResult (.HitResult (Utilities|Struct|BreakPredictProjectilePathResult _predictresult)))))))
      (Variables|Default|Setimpactpoint (Math|Vector|MakeVector (Math|Float|Clamp(Float) (.X (Math|Vector|BreakVector _output_get_3)) (Variables|Default|GetCourminX) (Variables|Default|GetCourMaxX)) (Math|Float|Clamp(Float) (.Y (Math|Vector|BreakVector _output_get_3)) (Variables|Default|GetCourMinY) (Variables|Default|GetCourMaxY)) (Variables|Default|GetCourtZ)))
      (bind _outactors_2 (Actor|GetAllActorsOfClass "/Game/BP_ScoreManager.BP_ScoreManager_C"))
      (CallFunction|RemoveAI)
      (Development|PrintString "check appele")
      (if (Variables|/Game/BP_ScoreManager.BP_ScoreManager_C|GetNextTeam (Utilities|Array|Get(acopy) _outactors_2))
        (Rendering|Debug|DrawDebugSphere (Variables|Default|Getimpactpoint) 3e+01 50 "(R=1.000000,G=0.000000,B=0.095176,A=1.000000)" 0.1)
        (bind _outactors_3 (Actor|GetAllActorsOfClass "/Game/ThirdPerson/Blueprints/BP_Player.BP_Player_C"))
        (bind _outactors_4 (Actor|GetAllActorsOfClass "/Game/ThirdPerson/Blueprints/BP_AIFriend.BP_AIFriend_C"))
        (Default|AIClearorder (Utilities|Array|Get(acopy) _outactors_4))
        (bind _output_get_4 (LocalVariables|Setcloseallie (Utilities|Array|Get(acopy) _outactors_4)))
        (if (> (Math|Vector|Distance(Vector) (Transformation|GetActorLocation (Utilities|Array|Get(acopy) _outactors_3)) (Variables|Default|Getimpactpoint)) (Math|Vector|Distance(Vector) (Transformation|GetActorLocation (Utilities|Array|Get(acopy) _outactors_4)) (Variables|Default|Getimpactpoint)))
          (Variables|/Game/ThirdPerson/Blueprints/BP_AIFriend.BP_AIFriend_C|SetHasorder _output_get_4 true)
          (Default|AISetGoal _output_get_4 (Math|Vector|SelectVector (.ProjectedLocation (AI|Navigation|ProjectPointtoNavigation (Variables|Default|Getimpactpoint) 0 0 "0, 0, 0")) (Variables|Default|Getimpactpoint) (.ReturnValue (AI|Navigation|ProjectPointtoNavigation (Variables|Default|Getimpactpoint) 0 0 "0, 0, 0"))))
          (Development|PrintString "friend move")
          (else
            (Development|PrintString (Utilities|String|ToString(Float) (Math|Vector|Distance(Vector) (Transformation|GetActorLocation (Utilities|Array|Get(acopy) _outactors_3)) (Variables|Default|Getimpactpoint))))))
        (else
          (bind _outactors_5 (Actor|GetAllActorsOfClass "/Game/ThirdPerson/Blueprints/BP_AI.BP_AI_C"))
          (for _array_element _outactors_5
            (Default|AIClearorder _array_element)
            (if (> (LocalVariables|GetBestDist) (Math|Vector|Distance(Vector) (Transformation|GetActorLocation _array_element) (Variables|Default|Getimpactpoint)))
              (LocalVariables|SetBestDist (Math|Vector|Distance(Vector) (Transformation|GetActorLocation _array_element) (Variables|Default|Getimpactpoint)))
              (bind _output_get_5 (Variables|Default|SetBestAI _array_element))))
          (bind _output_get_6 (LocalVariables|SetCLoseAI _output_get_5))
          (Variables|/Game/ThirdPerson/Blueprints/BP_AI.BP_AI_C|SetHasOrder _output_get_6 true)
          (Rendering|Debug|DrawDebugSphere (Variables|Default|Getimpactpoint) 3e+01 50 "(R=1.000000,G=0.000000,B=0.095176,A=1.000000)" 1.0)
          (Default|AISetGoal _output_get_6 (Math|Vector|SelectVector (.ProjectedLocation (AI|Navigation|ProjectPointtoNavigation (Variables|Default|Getimpactpoint) 0 0 "0, 0, 0")) (Variables|Default|Getimpactpoint) (.ReturnValue (AI|Navigation|ProjectPointtoNavigation (Variables|Default|Getimpactpoint) 0 0 "0, 0, 0")))))))))

(fn CalculballimpactAI
  (bind _outactors (Actor|GetAllActorsOfClass "/Game/BP_Ball.BP_Ball_C"))
  (if (> (Utilities|Array|Length _outactors) 0)
    (bind _output_get (Variables|Default|SetBallref (Utilities|Array|Get(acopy) _outactors)))
    (bind _output_get_2 (Variables|Default|SetBallMesh (Actor|GetComponentbyClass _output_get "/Script/Engine.StaticMeshComponent")))
    (if (Physics|IsSimulatingPhysics _output_get_2 "None")
      (bind _returnvalue (Physics|GetPhysicsLinearVelocity (Variables|Default|GetBallMesh) "None"))
      (bind _predictresult (Class|GameplayStatics|BlueprintPredictProjectilePathAdvanced (Utilities|Struct|MakePredictProjectilePathParams (Transformation|GetWorldLocation (Variables|Default|GetBallMesh)) _returnvalue true 15.0 4.0 true "ECC_Visibility" "ObjectTypeQuery1" (Utilities|Array|MakeArray (Variables|Default|GetBallref)) 3e+01)))
      (bind _output_get_3 (Variables|Default|SetImpactraw (Math|Vector|SelectVector (.Location (Collision|BreakHitResult (.HitResult (Utilities|Struct|BreakPredictProjectilePathResult _predictresult)))) (.Location (Utilities|Struct|BreakPredictProjectilePathPointData (.LastTraceDestination (Utilities|Struct|BreakPredictProjectilePathResult _predictresult)))) (.bBlockingHit (Collision|BreakHitResult (.HitResult (Utilities|Struct|BreakPredictProjectilePathResult _predictresult)))))))
      (Variables|Default|Setimpactpoint (Math|Vector|MakeVector (Math|Float|Clamp(Float) (.X (Math|Vector|BreakVector _output_get_3)) (Variables|Default|GetCourminX) (Variables|Default|GetCourMaxX)) (Math|Float|Clamp(Float) (.Y (Math|Vector|BreakVector _output_get_3)) (Variables|Default|GetCourMinY) (Variables|Default|GetCourMaxY)) (Variables|Default|GetCourtZ)))
      (bind _outactors_2 (Actor|GetAllActorsOfClass "/Game/ThirdPerson/Blueprints/BP_AI.BP_AI_C"))
      (for _array_element _outactors_2
        (Default|AIClearorder _array_element)
        (if (> (LocalVariables|GetBest%20Dist) (Math|Vector|Distance(Vector) (Transformation|GetActorLocation _array_element) (Variables|Default|Getimpactpoint)))
          (LocalVariables|SetBest%20Dist (Math|Vector|Distance(Vector) (Transformation|GetActorLocation _array_element) (Variables|Default|Getimpactpoint)))
          (bind _output_get_4 (Variables|Default|SetBestAI _array_element))))
      (bind _output_get_5 (LocalVariables|SetCLose%20AI _output_get_4))
      (Variables|/Game/ThirdPerson/Blueprints/BP_AI.BP_AI_C|SetHasOrder _output_get_5 true)
      (Rendering|Debug|DrawDebugSphere (Variables|Default|Getimpactpoint) 3e+01 50 "(R=1.000000,G=0.000000,B=0.095176,A=1.000000)" 1.0)
      (Default|AISetGoal _output_get_5 (Math|Vector|SelectVector (.ProjectedLocation (AI|Navigation|ProjectPointtoNavigation (Variables|Default|Getimpactpoint) 0 0 "0, 0, 0")) (Variables|Default|Getimpactpoint) (.ReturnValue (AI|Navigation|ProjectPointtoNavigation (Variables|Default|Getimpactpoint) 0 0 "0, 0, 0")))))))

(fn CalculeballImpactAIAillier
  (bind _outactors (Actor|GetAllActorsOfClass "/Game/BP_Ball.BP_Ball_C"))
  (if (> (Utilities|Array|Length _outactors) 0)
    (bind _output_get (Variables|Default|SetBallref (Utilities|Array|Get(acopy) _outactors)))
    (bind _output_get_2 (Variables|Default|SetBallMesh (Actor|GetComponentbyClass _output_get "/Script/Engine.StaticMeshComponent")))
    (if (Physics|IsSimulatingPhysics _output_get_2 "None")
      (bind _returnvalue (Physics|GetPhysicsLinearVelocity (Variables|Default|GetBallMesh) "None"))
      (bind _predictresult (Class|GameplayStatics|BlueprintPredictProjectilePathAdvanced (Utilities|Struct|MakePredictProjectilePathParams (Transformation|GetWorldLocation (Variables|Default|GetBallMesh)) _returnvalue true 15.0 4.0 true "ECC_Visibility" "ObjectTypeQuery1" (Utilities|Array|MakeArray (Variables|Default|GetBallref)) 3e+01)))
      (bind _output_get_3 (Variables|Default|SetImpactraw (Math|Vector|SelectVector (.Location (Collision|BreakHitResult (.HitResult (Utilities|Struct|BreakPredictProjectilePathResult _predictresult)))) (.Location (Utilities|Struct|BreakPredictProjectilePathPointData (.LastTraceDestination (Utilities|Struct|BreakPredictProjectilePathResult _predictresult)))) (.bBlockingHit (Collision|BreakHitResult (.HitResult (Utilities|Struct|BreakPredictProjectilePathResult _predictresult)))))))
      (Variables|Default|Setimpactpoint (Math|Vector|MakeVector (Math|Float|Clamp(Float) (.X (Math|Vector|BreakVector _output_get_3)) (Variables|Default|GetCourminX) (Variables|Default|GetCourMaxX)) (Math|Float|Clamp(Float) (.Y (Math|Vector|BreakVector _output_get_3)) (Variables|Default|GetCourMinY) (Variables|Default|GetCourMaxY)) (Variables|Default|GetCourtZ)))
      (Rendering|Debug|DrawDebugSphere (Variables|Default|Getimpactpoint) 3e+01 50 "(R=1.000000,G=0.000000,B=0.095176,A=1.000000)" 0.1)
      (bind _outactors_2 (Actor|GetAllActorsOfClass "/Game/ThirdPerson/Blueprints/BP_Player.BP_Player_C"))
      (bind _outactors_3 (Actor|GetAllActorsOfClass "/Game/ThirdPerson/Blueprints/BP_AIFriend.BP_AIFriend_C"))
      (Default|AIClearorder (Utilities|Array|Get(acopy) _outactors_3))
      (bind _output_get_4 (LocalVariables|SetCloseallie (Utilities|Array|Get(acopy) _outactors_3)))
      (if (not (> (Math|Vector|Distance(Vector) (Transformation|GetActorLocation (Utilities|Array|Get(acopy) _outactors_3)) (Variables|Default|Getimpactpoint)) (Math|Vector|Distance(Vector) (Transformation|GetActorLocation (Utilities|Array|Get(acopy) _outactors_2)) (Variables|Default|Getimpactpoint))))
        (Variables|/Game/ThirdPerson/Blueprints/BP_AIFriend.BP_AIFriend_C|SetHasorder _output_get_4 true)
        (Default|AISetGoal _output_get_4 (Math|Vector|SelectVector (.ProjectedLocation (AI|Navigation|ProjectPointtoNavigation (Variables|Default|Getimpactpoint) 0 0 "0, 0, 0")) (Variables|Default|Getimpactpoint) (.ReturnValue (AI|Navigation|ProjectPointtoNavigation (Variables|Default|Getimpactpoint) 0 0 "0, 0, 0"))))))))

(fn RemoveAI
  (bind _outactors (Actor|GetAllActorsOfClass "/Game/ThirdPerson/Blueprints/BP_AIFriend.BP_AIFriend_C"))
  (Variables|/Game/ThirdPerson/Blueprints/BP_AIFriend.BP_AIFriend_C|SetHasorder (Utilities|Array|Get(acopy) _outactors) false)
  (bind _outactors_2 (Actor|GetAllActorsOfClass "/Game/ThirdPerson/Blueprints/BP_AI.BP_AI_C"))
  (for _array_element _outactors_2
    (Variables|/Game/ThirdPerson/Blueprints/BP_AI.BP_AI_C|SetHasOrder _array_element false)))